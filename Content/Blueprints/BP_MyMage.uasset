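; BP_MyMage is a mage unit Blueprint with team, health and movement speed settings.
; BeginPlay applies movement speed, initializes the Health1 component from the Health variable and prints the result.
; A separate function, not called in this file, gathers all Unit actors, stores those on other teams in FoundUnits and prints their attack types.
; The random team assignment is disconnected and never runs.
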(event EventBeginPlay
  (bind _health1 (Variables|Default|GetHealth1))
  (Variables|/Script/Engine.CharacterMovementComponent|SetMaxWalkSpeed (Variables|Character|GetCharacterMovement) (Variables|Default|GetMovementSpeed))
  (Variables|/Script/BattleSimulator.HealthComponent|SetDefaultHealth _health1 (Variables|Default|GetHealth))
  (bind _output_get (Variables|/Script/BattleSimulator.HealthComponent|SetHealth _health1 (Variables|/Script/BattleSimulator.HealthComponent|GetDefaultHealth _health1)))
  (Development|PrintString (Utilities|String|ToString(Float) _output_get)))

(event Collision|EventActorBeginOverlap
  (params (OtherActor :type Actor%20Object%20Reference)))

(event EventTick
  (params (DeltaSeconds :type Float%20%28single-precision%29)))

(fn ConstructionScript)

(fn FindingEnemyUnitsandStoringinArray
  (bind _outactors (Actor|GetAllActorsOfClass "/Script/BattleSimulator.Unit"))
  (for _array_element _outactors
    (Utilities|Array|Add (Variables|Default|GetFoundActors) _array_element))
  (for _array_element_2 (Variables|Default|GetFoundActors)
    (bind _asunit (Utilities|Casting|CastToUnit _array_element_2)
      (:then
        (if (not (== (Variables|/Script/BattleSimulator.Unit|GetTeam _asunit) (Variables|Default|GetTeam)))
          (Utilities|Array|Add (Variables|Default|GetFoundUnits) _asunit)))
      (:CastFailed
        (Development|PrintString "failed"))))
  (for _array_element_3 (Variables|Default|GetFoundUnits)
    (Development|PrintString (Utilities|String|EnumtoString (Variables|/Script/BattleSimulator.Unit|GetAttackType _array_element_3)))))